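; BP_Bullet is a projectile actor that flies straight along its facing direction and knocks down BP_Target actors it hits.
; Tick calls MoveForward, which applies a swept world offset scaled by Speed and delta time, with no projectile movement component involved.
; A Sphere1 hit calls DownEvent on a target, then destroys the bullet whatever it struck.
; A timer started on BeginPlay also destroys it after a short lifetime.
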(event OnComponentHit(Sphere1)
  (params (HitComponent :type Primitive%20Component%20Object%20Reference) (OtherActor :type Actor%20Object%20Reference) (OtherComp :type Primitive%20Component%20Object%20Reference) (NormalImpulse :type Vector :default "0, 0, 0") (Hit :type Hit%20Result%20Structure%20%28by%20ref%29))
  (Utilities|FlowControl|Sequence
    (:then_0
      (bind _asbp_target (Utilities|Casting|CastToBP_Target OtherActor))
      (Default|DownEvent _asbp_target))
    (:then_1
      (Actor|DestroyActor))))

(event Custom|DestroybyTime
  (Actor|DestroyActor))

(event EventBeginPlay
  (Utilities|Time|SetTimerbyEvent (delegate Custom|DestroybyTime) 3.0))

(event Collision|EventActorBeginOverlap
  (params (OtherActor :type Actor%20Object%20Reference)))

(event EventTick
  (params (DeltaSeconds :type Float%20%28single-precision%29))
  (CallFunction|MoveForward DeltaSeconds (Variables|Default|Getspeed)))

(fn ConstructionScript)

(fn MoveForward
  (params (deltaTime :type Float%20%28double-precision%29) (speed :type Float%20%28double-precision%29))
  (Transformation|AddActorWorldOffset (* (* deltaTime speed) (Math|Vector|GetForwardVector (Transformation|GetActorRotation))) true))